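; Pickup actor that the player collects by overlapping its hitbox, incrementing the pawn's PickupsTaken count.
; It destroys itself when collected or when its hitbox stops overlapping a component tagged ActiveArea.
; On destruction for either reason, it increments the game mode's PickupsToSpawn counter, apparently to queue a replacement.
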(event OnComponentEndOverlap(Hitbox)
  (params (OverlappedComponent :type Primitive%20Component%20Object%20Reference) (OtherActor :type Actor%20Object%20Reference) (OtherComp :type Primitive%20Component%20Object%20Reference) (OtherBodyIndex :type Integer))
  (if (Components|ComponentHasTag OtherComp "ActiveArea")
    (Actor|DestroyActor)))

(event OnComponentBeginOverlap(Hitbox)
  (params (OverlappedComponent :type Primitive%20Component%20Object%20Reference) (OtherActor :type Actor%20Object%20Reference) (OtherComp :type Primitive%20Component%20Object%20Reference) (OtherBodyIndex :type Integer) (bFromSweep :type Boolean) (SweepResult :type Hit%20Result%20Structure%20%28by%20ref%29))
  (if (Components|ComponentHasTag OtherComp "Player")
    (bind _asmy_pawn (Utilities|Casting|CastToMyPawn OtherActor))
    (Variables|/Game/Blueprints/MyPawn.MyPawn_C|SetpickupsTaken _asmy_pawn (+ (Variables|/Game/Blueprints/MyPawn.MyPawn_C|GetpickupsTaken _asmy_pawn) 1))
    (Actor|DestroyActor)))

(event EventDestroyed
  (bind _asmy_game_mode (Utilities|Casting|CastToMyGameMode (Game|GetGameMode)))
  (Variables|/Game/Blueprints/MyGameMode.MyGameMode_C|SetpickupsToSpawn _asmy_game_mode (+ (Variables|/Game/Blueprints/MyGameMode.MyGameMode_C|GetpickupsToSpawn _asmy_game_mode) 1)))

(fn ConstructionScript)