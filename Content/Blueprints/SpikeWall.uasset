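; SpikeWall is a hazard actor that kills the player and clears destroyable actors it touches.
; On BeginPlay it places itself at a fixed X offset from the player pawn's Sphere component.
; Every tick it moves along negative X at the game mode's PanSpeed.
; On overlap it sets a MyPawn's HitPoints to zero, or calls DestroyActor on a DestroyableActor.
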(event EventBeginPlay
  (bind _asmy_pawn (Utilities|Casting|CastToMyPawn (Game|Player|GetPlayerPawn 0)))
  (Transformation|SetWorldLocation (Variables|Default|GetDefaultSceneRoot) (+ "1050.000000,0,0.000000" (Transformation|GetWorldLocation (Variables|/Game/Blueprints/MyPawn.MyPawn_C|GetSphere _asmy_pawn))) false false))

(event Collision|EventActorBeginOverlap
  (params (OtherActor :type Actor%20Object%20Reference))
  (bind _asmy_pawn (Utilities|Casting|CastToMyPawn OtherActor)
    (:then
      (Variables|/Game/Blueprints/MyPawn.MyPawn_C|SethitPoints _asmy_pawn 0))
    (:CastFailed
      (bind _asdestroyable_actor (Utilities|Casting|CastToDestroyableActor OtherActor))
      (Actor|DestroyActor _asdestroyable_actor))))

(event EventTick
  (params (DeltaSeconds :type Float%20%28single-precision%29))
  (bind _asmy_game_mode (Utilities|Casting|CastToMyGameMode (Game|GetGameMode)))
  (Transformation|AddRelativeLocation (Variables|Default|GetDefaultSceneRoot) (* (Variables|/Game/Blueprints/MyGameMode.MyGameMode_C|GetPanSpeed _asmy_game_mode) DeltaSeconds "-1.000000,0,0") false false))

(fn ConstructionScript)