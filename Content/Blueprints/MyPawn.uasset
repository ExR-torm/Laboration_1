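; Player pawn for an auto-scrolling game, moving a Sphere inside a play area that pans along -X.
; Each Tick clamps the Sphere to camera-relative borders, then pans Camera and Sphere by the GameMode's PanSpeed.
; Axis input sets a normalized DesiredVelocity that Velocity lerps toward, applied as separate swept X and Y moves.
; Tick also draws debug view bounds and ActiveArea; Hurt subtracts HitPoints and pauses the game at zero.
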(event EventTick
  (params (DeltaSeconds :type Float%20%28single-precision%29))
  (bind _activearea (Variables|Default|GetActiveArea))
  (bind _sphere (Variables|Default|GetSphere))
  (bind _camera (Variables|Default|GetCamera))
  (bind _sphere_2 (Variables|Default|GetSphere))
  (bind _camera_2 (Variables|Default|GetCamera))
  (bind _returnvalue (Transformation|GetWorldLocation _camera_2))
  (bind _returnvalue_2 (Math|Vector|GetForwardVector _camera_2))
  (bind _returnvalue_3 (Transformation|GetWorldLocation _sphere))
  (bind _returnvalue_4 (Transformation|GetWorldLocation _camera))
  (bind _returnvalue_5 (- _returnvalue_3 _returnvalue_4))
  (bind (_x _y _z) (Math|Vector|BreakVector _returnvalue_5))
  (Variables|Default|SetdeltaSeconds DeltaSeconds)
  ;[1 1 1] Clamp Player To Borders
  (Transformation|SetWorldLocation _sphere (+ (Math|Vector|MakeVector (Math|Float|Clamp(Float) _x -1.12e+03 1165.0) (Math|Float|Clamp(Float) _y -6.1e+02 625.0) _z) _returnvalue_4) false false)
  ;[1 1 1] Pan Play Area
  (bind _asmy_game_mode (Utilities|Casting|CastToMyGameMode (Game|GetGameMode)))
  (Transformation|AddRelativeLocation (Variables|Default|GetCamera) (* (Variables|/Game/Blueprints/MyGameMode.MyGameMode_C|GetPanSpeed _asmy_game_mode) (Variables|Default|GetdeltaSeconds) "-1.000000,0,0") false false)
  (Transformation|AddRelativeLocation (Variables|Default|GetSphere) (* (Variables|/Game/Blueprints/MyGameMode.MyGameMode_C|GetPanSpeed _asmy_game_mode) (Variables|Default|GetdeltaSeconds) "-1.000000,0,0") true false)
  ;[1 1 1] Player Movement
  (bind _output_get (Variables|Default|Setvelocity (Math|Vector|Lerp(Vector) (Variables|Default|Getvelocity) (Variables|Default|GetdesiredVelocity) (* 7.5 (Variables|Default|GetdeltaSeconds)))))
  (Transformation|AddRelativeLocation _sphere_2 (* (* _output_get (Variables|Default|Getspeed) (Variables|Default|GetspeedModifier) (Variables|Default|GetdeltaSeconds)) "1.000000,0,0") true false)
  (Transformation|AddRelativeLocation _sphere_2 (* (* _output_get (Variables|Default|Getspeed) (Variables|Default|GetspeedModifier) (Variables|Default|GetdeltaSeconds)) "0,1.000000,0") true false)
  (Rendering|Debug|DrawDebugBox (Transformation|GetWorldLocation _activearea) (Components|Box|GetScaledBoxExtent _activearea) "(R=0.441913,G=0.422180,B=1.000000,A=1.000000)" (Transformation|GetWorldRotation _activearea) 0.1 1e+01)
  (Rendering|Debug|DrawDebugArrow _returnvalue (+ _returnvalue (* (Math|Vector|RotateVector _returnvalue_2 "30.000000, 0,16.875000") (Class|KismetSystemLibrary|MakeLiteralInteger 2600))) 5.0 "(R=0.034150,G=1.000000,B=0.000000,A=1.000000)" 0.05 7.5)
  (Rendering|Debug|DrawDebugArrow _returnvalue (+ _returnvalue (* (Math|Vector|RotateVector _returnvalue_2 "30.000000, 0,-16.875000") (Class|KismetSystemLibrary|MakeLiteralInteger 2600))) 5.0 "(R=0.034150,G=1.000000,B=0.000000,A=1.000000)" 0.05 7.5)
  (Rendering|Debug|DrawDebugArrow _returnvalue (+ _returnvalue (* (Math|Vector|RotateVector _returnvalue_2 "-30.000000, 0,16.875000") (Class|KismetSystemLibrary|MakeLiteralInteger 2600))) 5.0 "(R=0.034150,G=1.000000,B=0.000000,A=1.000000)" 0.05 7.5)
  (Rendering|Debug|DrawDebugArrow _returnvalue (+ _returnvalue (* (Math|Vector|RotateVector _returnvalue_2 "-30.000000, 0,-16.875000") (Class|KismetSystemLibrary|MakeLiteralInteger 2600))) 5.0 "(R=0.034150,G=1.000000,B=0.000000,A=1.000000)" 0.05 7.5))

(event Input|AxisEvents|InputAxisLeft
  (params (AxisValue :type Float%20%28single-precision%29))
  ;[1 1 1] Set Desired Velocity
  (Variables|Default|SetdesiredVelocity (Math|Vector|Normalize (Math|Vector|MakeVector (+ AxisValue (stale Input|AxisEvents|InputAxisRight AxisValue)) (+ (stale Input|AxisEvents|InputAxisUp AxisValue) (stale Input|AxisEvents|InputAxisDown AxisValue)) 0.0) 0.1)))

(event Input|AxisEvents|InputAxisRight
  (params (AxisValue :type Float%20%28single-precision%29))
  ;[1 1 1] Set Desired Velocity
  (Variables|Default|SetdesiredVelocity (Math|Vector|Normalize (Math|Vector|MakeVector (+ (stale Input|AxisEvents|InputAxisLeft AxisValue) AxisValue) (+ (stale Input|AxisEvents|InputAxisUp AxisValue) (stale Input|AxisEvents|InputAxisDown AxisValue)) 0.0) 0.1)))

(event Input|AxisEvents|InputAxisDown
  (params (AxisValue :type Float%20%28single-precision%29))
  ;[1 1 1] Set Desired Velocity
  (Variables|Default|SetdesiredVelocity (Math|Vector|Normalize (Math|Vector|MakeVector (+ (stale Input|AxisEvents|InputAxisLeft AxisValue) (stale Input|AxisEvents|InputAxisRight AxisValue)) (+ (stale Input|AxisEvents|InputAxisUp AxisValue) AxisValue) 0.0) 0.1)))

(event Input|AxisEvents|InputAxisUp
  (params (AxisValue :type Float%20%28single-precision%29))
  ;[1 1 1] Set Desired Velocity
  (Variables|Default|SetdesiredVelocity (Math|Vector|Normalize (Math|Vector|MakeVector (+ (stale Input|AxisEvents|InputAxisLeft AxisValue) (stale Input|AxisEvents|InputAxisRight AxisValue)) (+ AxisValue (stale Input|AxisEvents|InputAxisDown AxisValue)) 0.0) 0.1)))

(fn ConstructionScript)

(fn Hurt
  (params (Damage :type Integer))
  (bind _output_get (Variables|Default|SethitPoints (- (Variables|Default|GethitPoints) Damage)))
  (Game|SetGamePaused (<= _output_get 0)))