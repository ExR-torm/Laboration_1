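; Obstacle actor that damages the player on contact and recycles itself through the game mode's spawn queue.
; Its Hitbox destroys it after hurting a Player-tagged MyPawn or upon leaving an ActiveArea-tagged component.
; Destruction increments the game mode's obstacle spawn count.
; The construction script sizes the DoNotOverlap box, dividing by world scale to keep a fixed horizontal margin around the actor at any scale.
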(event OnComponentEndOverlap(Hitbox)
  (params (OverlappedComponent :type Primitive%20Component%20Object%20Reference) (OtherActor :type Actor%20Object%20Reference) (OtherComp :type Primitive%20Component%20Object%20Reference) (OtherBodyIndex :type Integer))
  ;[1 1 1 1 15] Upon leaving play-area: Destroy this actor.
  (if (Components|ComponentHasTag OtherComp "ActiveArea")
    (Actor|DestroyActor)))

(event OnComponentBeginOverlap(Hitbox)
  (params (OverlappedComponent :type Primitive%20Component%20Object%20Reference) (OtherActor :type Actor%20Object%20Reference) (OtherComp :type Primitive%20Component%20Object%20Reference) (OtherBodyIndex :type Integer) (bFromSweep :type Boolean) (SweepResult :type Hit%20Result%20Structure%20%28by%20ref%29))
  ;[1 1 1 1 15] Upon colliding with player: Hurt player & destroy this actor.
  (Utilities|IsValid OtherActor
    (:Is%20Valid
      (if (Components|ComponentHasTag OtherComp "Player")
        (bind _asmy_pawn (Utilities|Casting|CastToMyPawn OtherActor))
        (Default|Hurt _asmy_pawn 1)
        (Actor|DestroyActor)))))

(event EventDestroyed
  ;[1 1 1 1 15] Upon destruction: Increment spawn-queue for this actor-type by one.
  (bind _asmy_game_mode (Utilities|Casting|CastToMyGameMode (Game|GetGameMode)))
  (Math|Integer|IncrementInt (Variables|/Game/Blueprints/MyGameMode.MyGameMode_C|GetobstablesToSpawn _asmy_game_mode)))

(fn ConstructionScript
  ;[1 1 1 1 15] Upon construction: Set DoNotOverlap bounds to an absolute scale wider than this actor.
  (Components|Box|SetBoxExtent (Variables|Default|GetDoNotOverlap) (+ (/ "65.000000,65.000000,0" (Transformation|GetWorldScale (Variables|Default|GetDefaultSceneRoot))) "50.000000,50.000000,50.000000") true))