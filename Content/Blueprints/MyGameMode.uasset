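; Game mode for a timed dodge-and-pickup game: creates the player UI, tracks win time and ramps PanSpeed with a smootherstep curve.
; BeginPlay seeds five areas along negative X; Tick retries spawning every half-second via Delay, growing the queues periodically after winning.
; TrySpawn functions consume queue counters to place walls, obstacles and pickups randomly relative to the camera, skipping collisions.
; Walls and obstacles get random scales, then shrink to avoid blocking paths.
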(event EventBeginPlay
  ;[1 1 1 1 15] Create player-UI
  (bind _returnvalue (UserInterface|CreateWidget "/Game/Blueprints/PlayerUI.PlayerUI_C"))
  (UserInterface|Viewport|AddtoViewport _returnvalue 0)
  ;[1 1 1 1 15] Try to spawn up to 5 semi-evenly spaced objects of all types
  (for _index (range 1 5)
    (CallFunction|TrySpawnWall (Class|KismetMathLibrary|MakeBoxSphereBounds (Math|Vector|MakeVector (Math|Conversions|ToFloat(Integer) (* _index -1000)) 0.0 0.0) "500.000000,600.000000, 0" 0.0))
    (CallFunction|TrySpawnObstacle (Class|KismetMathLibrary|MakeBoxSphereBounds (Math|Vector|MakeVector (Math|Conversions|ToFloat(Integer) (* _index -1000)) 0.0 0.0) "500.000000,600.000000, 0" 0.0))
    (CallFunction|TrySpawnPickup (Class|KismetMathLibrary|MakeBoxSphereBounds (Math|Vector|MakeVector (Math|Conversions|ToFloat(Integer) (* _index -1000)) 0.0 0.0) "500.000000,600.000000, 0" 0.0))))

(event EventTick
  (params (DeltaSeconds :type Float%20%28single-precision%29))
  (bind _spawnablearea (Variables|Default|GetspawnableArea))
  ;[1 1 1 1 15] Set current progression from start to end
  (bind _output_get (Variables|Default|SettotalTime (+ DeltaSeconds (Variables|Default|GettotalTime))))
  (bind _output_get_2 (Variables|Default|Setprogress (/ _output_get (Variables|Default|GetgameLength))))
  ;[1 1 1 1 15] Smoothly interpolate from start-panSpeed (S0) to end-panSpeed (S1)
  (Variables|Default|SetpanSpeed (+ (* (* (Math|Float|Power _output_get_2 3.0) (+ (* _output_get_2 (- (* _output_get_2 6.0) 15.0)) 1e+01)) 8e+02) 2.5e+02))
  (Variables|Default|SethasWon (>= (Variables|Default|GettotalTime) (Variables|Default|GetgameLength)))
  ;[1 1 1 1 15] Try to spawn new set of objects every half-second.
  (Utilities|FlowControl|Delay 0.5)
  (CallFunction|TrySpawnWall _spawnablearea)
  (CallFunction|TrySpawnObstacle _spawnablearea)
  (CallFunction|TrySpawnPickup _spawnablearea)
  ;[1 1 1 1 15] Occasionally increase total object-count if end of game has been reached.
  (if (Variables|Default|GethasWon)
    (Utilities|FlowControl|Delay 4e+01)
    (Math|Integer|IncrementInt (Variables|Default|GetobstablesToSpawn)
      (:%20%20
        (Math|Integer|IncrementInt (Variables|Default|GetwallsToSpawn)
          (:%20%20
            (Math|Integer|IncrementInt (Variables|Default|GetpickupsToSpawn))))))))

(fn ConstructionScript)

(fn TrySpawnWall
  (params (randomSpawnBounds :type Box%20Sphere%20Bounds%20Structure))
  (bind _returnvalue (Math|Random|RandomFloatinRange 1.0 8.0))
  (bind (_origin _boxextent) (Math|BoxSphereBounds|BreakBoxSphereBounds randomSpawnBounds))
  ;[1 1 1 1 15] Check if a wall is queued to spawn
  (if (> (Variables|Default|GetwallsToSpawn) 0)
    ;[1 1 1 1 15] Get player-pos
    (bind _asmy_pawn (Utilities|Casting|CastToMyPawn (Game|Player|GetPlayerPawn 0)))
    (bind _returnvalue_2 (Game|SpawnActorfromClass "/Game/Blueprints/Wall.Wall_C" (Math|Transform|MakeTransform (* (+ (Transformation|GetWorldLocation (Variables|/Game/Blueprints/MyPawn.MyPawn_C|GetCamera _asmy_pawn)) (Math|Random|RandomPointinBoundingBox _origin _boxextent)) "1.000000,1.000000,0") "0, 0, 0" (Math|Vector|MakeVector (Math|Random|RandomFloatinRange 0.25 (- 7.0 (/ _returnvalue 1.25))) _returnvalue (Math|Random|RandomFloatinRange 4.0 12.0))) "DontSpawnIfColliding" 0 0))
    ;[1 1 1 1 15] Shorten spawn-queue by one
    (Math|Integer|DecrementInt (Variables|Default|GetwallsToSpawn)
      (:%20%20
        ;[1 1 1 1 15] Scale wall down to minimize chance of fully blocking the player's path
        (Utilities|IsValid _returnvalue_2
          (:Is%20Valid
            (Transformation|SetActorRelativeScale3D _returnvalue_2 (* (Class|Actor|GetActorRelativeScale3D _returnvalue_2) "0.900000,0.800000,1.000000"))))))))

(fn TrySpawnObstacle
  (params (randomSpawnBounds :type Box%20Sphere%20Bounds%20Structure))
  (bind (_origin _boxextent) (Math|BoxSphereBounds|BreakBoxSphereBounds randomSpawnBounds))
  (bind _returnvalue (Math|Random|RandomFloatinRange 1.0 6.0))
  ;[1 1 1 1 15] Check if an obstacle is queued to spawn
  (if (> (Variables|Default|GetobstablesToSpawn) 0)
    ;[1 1 1 1 15] Get player-pos
    (bind _asmy_pawn (Utilities|Casting|CastToMyPawn (Game|Player|GetPlayerPawn 0)))
    (bind _returnvalue_2 (Game|SpawnActorfromClass "/Game/Blueprints/Obstacle.Obstacle_C" (Math|Transform|MakeTransform (* (+ (Transformation|GetWorldLocation (Variables|/Game/Blueprints/MyPawn.MyPawn_C|GetCamera _asmy_pawn)) (Math|Random|RandomPointinBoundingBox _origin _boxextent)) "1.000000,1.000000,0") "0, 0, 0" (Math|Vector|MakeVector (Math|Random|RandomFloatinRange 0.25 (- 6.0 (/ _returnvalue 1.25))) _returnvalue (Math|Random|RandomFloatinRange 4.0 1e+01))) "DontSpawnIfColliding" 0 0))
    ;[1 1 1 1 15] Shorten spawn-queue by one
    (Math|Integer|DecrementInt (Variables|Default|GetobstablesToSpawn)
      (:%20%20
        ;[1 1 1 1 15] Scale obstacle down to minimize chance of fully blocking the player's path
        (Utilities|IsValid _returnvalue_2
          (:Is%20Valid
            (Transformation|SetActorRelativeScale3D _returnvalue_2 (* (Class|Actor|GetActorRelativeScale3D _returnvalue_2) "0.900000,0.800000,1.000000"))))))))

(fn TrySpawnPickup
  (params (randomSpawnBounds :type Box%20Sphere%20Bounds%20Structure))
  (bind (_origin _boxextent) (Math|BoxSphereBounds|BreakBoxSphereBounds randomSpawnBounds))
  ;[1 1 1 1 15] Check if a pickup is queued to spawn
  (if (> (Variables|Default|GetpickupsToSpawn) 0)
    ;[1 1 1 1 15] Get player-pos
    (bind _asmy_pawn (Utilities|Casting|CastToMyPawn (Game|Player|GetPlayerPawn 0)))
    (Game|SpawnActorfromClass "/Game/Blueprints/Pickup.Pickup_C" (Math|Transform|MakeTransform (+ "0,0,295.000000" (* (+ (Transformation|GetWorldLocation (Variables|/Game/Blueprints/MyPawn.MyPawn_C|GetCamera _asmy_pawn)) (Math|Random|RandomPointinBoundingBox _origin _boxextent)) "1.000000,1.000000,0")) "0, 0, 0" "0.200000,0.200000,0.200000") "DontSpawnIfColliding" 0 0)
    ;[1 1 1 1 15] Shorten spawn-queue by one
    (Math|Integer|DecrementInt (Variables|Default|GetpickupsToSpawn))))